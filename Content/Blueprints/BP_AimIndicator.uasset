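; BP_AimIndicator is a particle-based aim pointer that changes color according to the kind of actor being aimed at.
; UpdateAimColor checks the hit actor's tags for Tortuga, Box or Door and sets the particle's Color parameter to the matching color, falling back to a default.
; An On/Off function activates or deactivates the pointer particle system.
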(fn `On/Off`
  (params (`On/Off` :type Boolean))
  (if `On/Off`
    (`ActorComponent.Activate` (`self.PS_Pointer`) false)
    (else
      (`ActorComponent.Deactivate` (`self.PS_Pointer`)))))

(fn `UpdateAimColor`
  (params (HitActor :type "Actor Object Reference"))
  (if (`self.ActorHasTag` HitActor "Tortuga")
    (`FXSystemComponent.SetColorParameter` (`self.PS_Pointer`) "Color" (`self.Tortuga_Color`))
    (elif (`self.ActorHasTag` HitActor "Box")
      (`FXSystemComponent.SetColorParameter` (`self.PS_Pointer`) "Color" (`self.Box_Color`))
      (elif (`self.ActorHasTag` HitActor "Door")
        (`FXSystemComponent.SetColorParameter` (`self.PS_Pointer`) "Color" (`self.Door_Color`))
        (else
          (`FXSystemComponent.SetColorParameter` (`self.PS_Pointer`) "Color" (`self.Defaul_Color`)))))))

(fn `UserConstructionScript`)