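; BP_EndDoor is a counter-gated door that can end the game with a win screen.
; AddToCounter raises Counter and calls TryToOpen, which, at MaxCount or above, sets rotation 20% from the starting yaw toward FinalRotation in one step, otherwise printing debug text.
; When Counter exactly equals MaxCount and IsEnd is set, a BP_ThirdPersonCharacter overlapping Collision gets the UW_Win widget and a mouse cursor.
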(event `self.ReceiveBeginPlay`
  (bind (_returnvalue_roll _returnvalue_pitch _returnvalue_yaw) (`KismetMathLibrary.BreakRotator` (`self.K2_GetActorRotation` self)))
  (set `self.DefaultRotation` (`KismetMathLibrary.MakeRotator` 0.0 0.0 _returnvalue_yaw)))

(event `self.Collision.OnComponentBeginOverlap`
  (params (OverlappedComponent :type "PrimitiveComponent Object Reference") (OtherActor :type "Actor Object Reference") (OtherComp :type "PrimitiveComponent Object Reference") (OtherBodyIndex :type Integer) (bFromSweep :type Boolean) (SweepResult :type "HitResult Structure (by ref)"))
  (if (== (`self.Counter`) (`self.MaxCount`))
    (if (== (`self.IsEnd`) true)
      (cast `/Game/ThirdPerson/Blueprints/BP_ThirdPersonCharacter` OtherActor)
      (bind _returnvalue (`|CreateWidget` "/Game/Blueprints/Widgets/UW_Win.UW_Win_C"))
      (`UserWidget.AddToViewport` _returnvalue 0)
      (set `PlayerController.bShowMouseCursor` true (`GameplayStatics.GetPlayerController` 0)))))

(fn `AddToCounter`
  (params (Value :type Integer))
  (set `self.Counter` (+ Value (`self.Counter`)))
  (`self.TryToOpen`))

(fn `TryToOpen`
  (if (>= (`self.Counter`) (`self.MaxCount`))
    (`self.K2_SetActorRotation` self (`KismetMathLibrary.RLerp` (`self.DefaultRotation`) (`self.FinalRotation`) 0.2) false)
    (else
      (`KismetSystemLibrary.PrintString` "Hello"))))

(fn `UserConstructionScript`)