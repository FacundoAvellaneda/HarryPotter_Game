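; Behavior tree task that picks the next patrol point for a BP_Enemy.
; On AI tick it reads the enemy's PatrollPoints, advances a stored waypoint index and wraps to zero at the end of the list.
; It writes that point as a vector to the selected blackboard key and finishes successfully, leaving movement itself outside this task.
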(event `self.ReceiveTickAI`
  (params (OwnerController :type "AIController Object Reference") (ControlledPawn :type "Pawn Object Reference") (DeltaSeconds :type "Float (single-precision)"))
  (bind _output (`|GetArrayItem` (`self.Waypoints`) (`self.CurrentWaypoint`)))
  (bind _asbp_enemy (cast `/Game/Blueprints/IA_Actors/BP_Enemy` ControlledPawn))
  (set `self.Waypoints` (`/Game/Blueprints/IA_Actors/BP_Enemy.PatrollPoints` _asbp_enemy))
  (set `self.CurrentWaypoint` (+ (`self.CurrentWaypoint`) 1))
  (if (== (`self.CurrentWaypoint`) (`KismetArrayLibrary.Array_Length` (`self.Waypoints`)))
    (set `self.CurrentWaypoint` 0)
    (`BTFunctionLibrary.SetBlackboardValueAsVector` (`self.BBSelector`) _output)
    (else
      (`BTFunctionLibrary.SetBlackboardValueAsVector` (`self.BBSelector`) _output)))
  (`self.FinishExecute` true))