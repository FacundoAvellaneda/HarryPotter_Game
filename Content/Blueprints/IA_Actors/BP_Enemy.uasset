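; AI enemy pawn that players can knock around and that reports perception results to its Blackboard.
; Every second Interact enables mesh physics, applies a horizontal impulse at the impact point and starts a Timeline blinking the dynamic material's BaseColor.
; The blink resets physics and color when TimeForReset is non-positive, though nothing here updates it; Tick's eight-second counter is separate.
; AIPerception writes sight state and TargetActor to the Blackboard.
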(event `/Game/ThirdPerson/Blueprints/BPI_Interactuable.Interact`
  (params (ImpactPoint :type "Vector Structure") (ImpactDirection :type "Vector Structure"))
  (set `self.InteractCounter` (+ (`self.InteractCounter`) 1))
  (set `self.IsMovible` true)
  (`PrimitiveComponent.SetMaterial` (`self.Mesh`) 0 (`self.DynamicMaterial`))
  (if (== (`self.InteractCounter`) 2)
    (set `self.InteractCounter` 0)
    (if (`self.IsMovible`)
      (`PrimitiveComponent.SetSimulatePhysics` (`self.Mesh`) true)
      (`PrimitiveComponent.AddImpulseAtLocation` (`self.Mesh`) (* (`KismetMathLibrary.MakeVector` (.x ImpactDirection) (.y ImpactDirection)) (`self.AddForce`)) ImpactPoint "None")
      (`self.StartBlink`)
      (else
        (`KismetSystemLibrary.PrintString` "no hago nada")))))

(event `self.ReceiveBeginPlay`
  (bind _returnvalue (`PrimitiveComponent.CreateDynamicMaterialInstance` (`self.Mesh`) 0 "/Game/Blueprints/BP_Materials/M_Tortuga.M_Tortuga" "None"))
  (bind _output_get (set `self.DynamicMaterial` _returnvalue))
  (bind _returnvalue_2 (`MaterialInstanceDynamic.K2_GetVectorParameterValue` _output_get "BaseColor"))
  (bind _output_get_2 (set `self.OriginalColor` _returnvalue_2)))

(event `StartBlink`
  (bind (_direction _alpha) (`Timeline|Timeline` :!label _label)
    (:`Update`
      (`MaterialInstanceDynamic.SetVectorParameterValue` (`self.DynamicMaterial`) "BaseColor" (`KismetMathLibrary.LinearColorLerp` (`self.MovibleColor`) (`self.OriginalColor`) _alpha))
      (if (>= 0.0 (`self.TimeForReset`))
        (set `self.CurrentTime` 0.0)
        (`PrimitiveComponent.SetSimulatePhysics` (`self.Mesh`) false)
        (`MaterialInstanceDynamic.SetVectorParameterValue` (`self.DynamicMaterial`) "BaseColor" (stale `self.ReceiveBeginPlay` _output_get_2))
        (set `self.IsMovible` false)
        (goto _label :!via `Stop`)))))

(event `self.ReceiveTick`
  (params (DeltaSeconds :type "Float (single-precision)"))
  (if (`self.IsMovible`)
    (bind _output_get (set `self.CurrentTime` (+ DeltaSeconds (`self.CurrentTime`))))
    (if (>= _output_get 8.0)
      (set `self.CurrentTime` 0.0))
    (else
      (set `self.CurrentTime` 0.0))))

(event `self.AIPerception.OnTargetPerceptionUpdated`
  (params (Actor :type "Actor Object Reference") (Stimulus :type "AIStimulus Structure"))
  (bind _asaicontroller (cast `AIController` (`self.GetController`)))
  (bind _output_get (set `self.ISeenPlayer` (`.bSuccessfullySensed` (break `AIStimulus` Stimulus))))
  (bind _returnvalue (`AIBlueprintHelperLibrary.GetBlackboard` _asaicontroller))
  (`BlackboardComponent.SetValueAsBool` _returnvalue (`KismetSystemLibrary.MakeLiteralName` (`KismetStringLibrary.Conv_StringToName` (`self.IseePlayer`))) _output_get)
  (`BlackboardComponent.SetValueAsObject` _returnvalue "TargetActor" Actor))

(fn `UserConstructionScript`)