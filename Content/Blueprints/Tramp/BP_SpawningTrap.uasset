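; BP_SpawningTrap is a trap actor that repeatedly fires projectiles, apparently fireballs given its throw sound.
; BeginPlay starts a looping timer at the FireRate interval that calls SpawnProyectil.
; While IsActivate is true, each tick of that timer spawns ProyectilClass at the SpawnPeroyectil component's world location and rotation and plays SC_ThrowFireball at the trap's location.
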(event `self.ReceiveBeginPlay`
  ;[1 1 1] Spawnear proyectil en base a un tiempo
  (`KismetSystemLibrary.K2_SetTimerDelegate` (delegate `SpawnProyectil`) (`self.FireRate`) true))

(event `SpawnProyectil`
  ;[1 1 1] Spawnear proyectil en base a un tiempo
  (if (== (`self.IsActivate`) true)
    (`|SpawnActorFromClass` (`self.ProyectilClass`) (`KismetMathLibrary.MakeTransform` (`SceneComponent.K2_GetComponentLocation` (`self.SpawnPeroyectil`)) (`SceneComponent.K2_GetComponentRotation` (`self.SpawnPeroyectil`))) "Undefined" "MultiplyWithRoot" null null)
    (`GameplayStatics.PlaySoundAtLocation` "/Game/Sounds/FireBall/SC_ThrowFireball.SC_ThrowFireball" (`self.K2_GetActorLocation`) (struct) 1.0 1.0 0.0 null null null null)))

(fn `UserConstructionScript`
  (`parent.UserConstructionScript`))